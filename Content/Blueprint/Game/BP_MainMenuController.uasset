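; Player controller for the main menu that creates and displays the main menu widget.
; On BeginPlay it calls ClientCreateUI, which adds the widget to the viewport, stores it and shows the mouse cursor.
; Pressing Space Bar switches the widget to its second page and sets UI-only input mode without locking the mouse.
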(event `self.ReceiveBeginPlay`
  ;[1 0 0] Comment
  (`self.ClientCreateUI`))

(event `ClientCreateUI`
  (bind _returnvalue (`|CreateWidget` "/Game/Blueprint/GameUI/WBP_MainMenuUI.WBP_MainMenuUI_C" self))
  (bind _output_get (set `self.UI_MainMenu` _returnvalue))
  (`UserWidget.AddToViewport` _output_get 0)
  (set `self.bShowMouseCursor` true))

(event `Key|SpaceBar`
  (params (Key :type "Key Structure"))
  (:`Pressed`
    (bind _ui_mainmenu (`self.UI_MainMenu`)
      (:`then`
        (`/Game/Blueprint/GameUI/WBP_MainMenuUI.SetActiveWidgetIndex` _ui_mainmenu 1)
        (`WidgetBlueprintLibrary.SetInputMode_UIOnlyEx` self null))
      (:`else`))))

(fn `UserConstructionScript`)