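; Game mode for a multiplayer FPS deathmatch that runs the round timer, spawning and scoring.
; PostLogin starts each controller's character spawn and registers its name and score, and RequestSpawn places BP_Attacker characters at player starts in round-robin order.
; A looping one-second timer pushes the countdown to every client and ends the game at zero.
; Kills add points and self-deaths subtract them, then all scores are sent to every controller.
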(event `self.ReceiveBeginPlay`
  (bind _outactors (`GameplayStatics.GetAllActorsOfClass` "/Script/Engine.PlayerStart"))
  (set `self.CharacterSpawnPoints` _outactors)
  (bind _returnvalue (`KismetSystemLibrary.K2_SetTimerDelegate` (delegate `Down`) 1.0 true))
  (set `self.CountDownTimer` _returnvalue))

(event `EndGame`
  (for _array_element (`self.AllPlayerContorller`)
    (`/Game/Blueprint/Game/BP_MultiFPSPlayerController.ClientEndGame` _array_element)))

(event `Down`
  (bind _result (`/Engine/EditorBlueprintResources/StandardMacros.DecrementInt` (`self.RoundTime`))
    (:`  `
      (for _array_element (`self.AllPlayerContorller`)
        (`/Game/Blueprint/Game/BP_MultiFPSPlayerController.ClientSetCountTime` _array_element _result))
      (if (<= (`self.RoundTime`) 0)
        (`KismetSystemLibrary.K2_ClearAndInvalidateTimerHandle` (`self.CountDownTimer`))
        (`self.EndGame`)))))

(event `self.K2_PostLogin`
  (params (NewPlayer :type "PlayerController Object Reference"))
  (bind _asbp_multi_fpsplayer_controller (cast `/Game/Blueprint/Game/BP_MultiFPSPlayerController` NewPlayer))
  (`/Game/Blueprint/Game/BP_MultiFPSPlayerController.StartSpawnCharacter` _asbp_multi_fpsplayer_controller)
  (`BlueprintMapLibrary.Map_Add` (`self.PlayerGameDataMap`) _asbp_multi_fpsplayer_controller (make `DeathMatchPlayerData` (`KismetStringLibrary.Conv_StringToName` (`KismetSystemLibrary.GetObjectName` _asbp_multi_fpsplayer_controller))))
  (bind _keys (`BlueprintMapLibrary.Map_Keys` (`self.PlayerGameDataMap`)))
  (set `self.AllPlayerContorller` _keys))

(event `RequestSpawn`
  (params (PlayerController :type "/Game/Blueprint/Game/BP_MultiFPSPlayerController Object Reference"))
  ;[1 1 1] 改变玩家生成位置
  (`/Game/Blueprint/Game/BP_MultiFPSPlayerController.SpawnPlayerCharacter` PlayerController "/Game/Blueprint/Player/BP_Attacker.BP_Attacker_C" (`self.GetTransform` (`|GetArrayItem` (`self.CharacterSpawnPoints`) (`self.SpawnPointIndex`))))
  (bind _output_get (set `self.SpawnPointIndex` (+ (`self.SpawnPointIndex`) 1)))
  (if (>= _output_get (`KismetArrayLibrary.Array_Length` (`self.CharacterSpawnPoints`)))
    (set `self.SpawnPointIndex` 0)))

(event `UpdateValues`
  (bind _keys (`BlueprintMapLibrary.Map_Keys` (`self.PlayerGameDataMap`)))
  (for _array_element _keys
    (bind _values (`BlueprintMapLibrary.Map_Values` (`self.PlayerGameDataMap`)))
    (`/Game/Blueprint/Game/BP_MultiFPSPlayerController.ClientUpdateValues` _array_element _values)))

(event `SelfDeath`
  (params (PlayerController :type "/Game/Blueprint/Game/BP_MultiFPSPlayerController Object Reference (by ref)"))
  (bind _playergamedatamap (`self.PlayerGameDataMap`))
  (bind (_value _returnvalue) (`BlueprintMapLibrary.Map_Find` _playergamedatamap PlayerController))
  (if _returnvalue
    (bind _output_get (set `self.ModifiedData` _value))
    (bind (_playername _playerscore) (break `DeathMatchPlayerData` _output_get))
    (bind _structout (setmembers `DeathMatchPlayerData` :`StructRef` _output_get :`PlayerName` _playername :`PlayerScore` (- _playerscore 10)))
    (`BlueprintMapLibrary.Map_Remove` _playergamedatamap PlayerController)
    (`BlueprintMapLibrary.Map_Add` _playergamedatamap PlayerController _structout)
    (`self.UpdateValues`)))

(event `KillAnother`
  (params (PlayerController :type "/Game/Blueprint/Game/BP_MultiFPSPlayerController Object Reference (by ref)"))
  (bind _playergamedatamap (`self.PlayerGameDataMap`))
  (bind (_value _returnvalue) (`BlueprintMapLibrary.Map_Find` _playergamedatamap PlayerController))
  (if _returnvalue
    (bind _output_get (set `self.ModifiedData` _value))
    (bind (_playername _playerscore) (break `DeathMatchPlayerData` _output_get))
    (bind _structout (setmembers `DeathMatchPlayerData` :`StructRef` _output_get :`PlayerName` _playername :`PlayerScore` (+ _playerscore 15)))
    (`BlueprintMapLibrary.Map_Remove` _playergamedatamap PlayerController)
    (`BlueprintMapLibrary.Map_Add` _playergamedatamap PlayerController _structout)
    (`self.UpdateValues`)))

(fn `UserConstructionScript`)