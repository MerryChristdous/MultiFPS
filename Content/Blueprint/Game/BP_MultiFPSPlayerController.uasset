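; Player controller for a multiplayer FPS deathmatch that handles spawning, death and the local player HUD.
; Deaths report victim and killer to BP_DeathMatchGameMode, destroy the pawn and request a respawn, which SpawnPlayerCharacter possesses.
; The local controller creates WBP_PlayerUI, then asks the server-only GameMode for scores, which ClientUpdateValues sorts and displays.
; Other events forward ammo, health and crosshair recoil to the HUD, store the countdown, or return to MainMenu.
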(event `ClientSetCountTime`
  (params (CountDown :type Integer))
  (set `self.CountDown` CountDown))

(event `self.DeathMatchDeath`
  (params (InstigatedBy :type "Controller Object Reference"))
  (bind _asbp_death_match_game_mode (cast `/Game/Blueprint/Game/BP_DeathMatchGameMode` (`GameplayStatics.GetGameMode`)))
  (`/Game/Blueprint/Game/BP_DeathMatchGameMode.SelfDeath` _asbp_death_match_game_mode self)
  (bind _asbp_multi_fpsplayer_controller (cast `/Game/Blueprint/Game/BP_MultiFPSPlayerController` InstigatedBy))
  (`/Game/Blueprint/Game/BP_DeathMatchGameMode.KillAnother` _asbp_death_match_game_mode _asbp_multi_fpsplayer_controller)
  (`self.K2_DestroyActor` (`self.K2_GetPawn`))
  (`KismetSystemLibrary.Delay` 0.2)
  (bind _asbp_death_match_game_mode_2 (cast `/Game/Blueprint/Game/BP_DeathMatchGameMode` (`GameplayStatics.GetGameMode`)))
  (`/Game/Blueprint/Game/BP_DeathMatchGameMode.RequestSpawn` _asbp_death_match_game_mode_2 self))

(event `ServerRequireUpdateValues`
  (bind _asbp_death_match_game_mode (cast `/Game/Blueprint/Game/BP_DeathMatchGameMode` (`GameplayStatics.GetGameMode`)))
  (`/Game/Blueprint/Game/BP_DeathMatchGameMode.UpdateValues` _asbp_death_match_game_mode))

(event `ClientUpdateValues`
  (params (Values :type "Array of DeathMatchPlayerData Structure"))
  ;[1 1 1] 每个客户端自己去更新UI数据
  (bind _output_get (set `self.Values` Values))
  (`MultiFPSLibrary.SortValues` _output_get)
  (bind _playerui (`self.PlayerUI`)
    (:`then`
      (`/Game/Blueprint/GameUI/WBP_PlayerUI.UpdateSortBox` _playerui (`self.Values`)))
    (:`else`)))

(event `SpawnPlayerCharacter`
  (params (Class :type "FPSBaseCharacter Class Reference") (SpawnTransform :type "Transform Structure"))
  (bind _returnvalue (`|SpawnActorFromClass` Class SpawnTransform "Undefined" "OverrideRootScale" null null))
  (`self.Possess` _returnvalue)
  (`self.ClientHideMouse`))

(event `ClientHideMouse`
  (`WidgetBlueprintLibrary.SetInputMode_GameOnly` self)
  (set `self.bShowMouseCursor` false))

(event `StartSpawnCharacter`
  (`KismetSystemLibrary.Delay` 1.0)
  (bind _asbp_death_match_game_mode (cast `/Game/Blueprint/Game/BP_DeathMatchGameMode` (`GameplayStatics.GetGameMode`)))
  (`/Game/Blueprint/Game/BP_DeathMatchGameMode.RequestSpawn` _asbp_death_match_game_mode self))

(event `ClientEndGame`
  (`GameplayStatics.OpenLevel` "MainMenu"))

(event `self.CreatePlayerUI`
  ;[1 1 1] UI
  (bind _playerui (`self.PlayerUI`)
    (:`then`
      (`Widget.RemoveFromParent` _playerui))
    (:`else`
      _))
  (if (`self.IsLocalPlayerController`)
    (bind _returnvalue (`|CreateWidget` "/Game/Blueprint/GameUI/WBP_PlayerUI.WBP_PlayerUI_C" self))
    (bind _output_get (set `self.PlayerUI` _returnvalue))
    (`UserWidget.AddToViewport` _output_get 0)
    ;;[1 1 1 1 15] UI被创建出来以后，去GameMode里更新所有玩家的数据，因为UI是在客户端上创建出来的，而GameMode只存在于服务器，所以要使用服务器事件
    (`self.ServerRequireUpdateValues`)))

(event `self.DoCrossHairRecoil`
  ;[1 1 1] UI
  (if (`KismetSystemLibrary.IsValid` (`self.PlayerUI`))
    (`/Game/Blueprint/GameUI/WBP_PlayerUI.DoCrosshairRecoil` (`self.PlayerUI`))))

(event `self.UpdateAmmoUI`
  (params (ClipCurrentAmmo :type Integer) (GunCurrentAmmo :type Integer))
  ;[1 1 1] UI
  (if (`KismetSystemLibrary.IsValid` (`self.PlayerUI`))
    (`/Game/Blueprint/GameUI/WBP_PlayerUI.UpdateAmmo` (`self.PlayerUI`) ClipCurrentAmmo GunCurrentAmmo)))

(event `self.UpdateHealthUI`
  (params (InHealth :type "Float (single-precision)") (InHealthPercent :type "Float (single-precision)") (InDamage :type "Float (single-precision)"))
  ;[1 1 1] UI
  (if (`KismetSystemLibrary.IsValid` (`self.PlayerUI`))
    (`/Game/Blueprint/GameUI/WBP_PlayerUI.UpdateHealth` (`self.PlayerUI`) InHealth InHealthPercent InDamage)))

(fn `UserConstructionScript`)